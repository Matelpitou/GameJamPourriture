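; BP_wall is an advancing hazard pawn that respawns the top-down player character on contact.
; On BeginPlay it saves its location, binds to the game mode's death reset and, if CanMove is set, uses AI MoveTo to walk toward Goal at AdvanceSpeed.
; Its Box overlap calls Respawn on the game mode, and the death-reset callback teleports the wall back to its saved start.
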(event `self.ReceiveBeginPlay`
  (set `self.Spawn transform` (`self.K2_GetActorLocation`))
  (bind _asbp_top_down_game_mode (cast `/Game/TopDown/Blueprints/BP_TopDownGameMode` (`GameplayStatics.GetGameMode`)))
  (add `/Game/TopDown/Blueprints/BP_TopDownGameMode.Reset_death` _asbp_top_down_game_mode (delegate `Reset death`))
  (`self.Wall advance`))

(event `Reset death`
  (`self.K2_SetActorLocation` self (`self.Spawn transform`) false true))

(event `self.Box.OnComponentBeginOverlap`
  (params (OverlappedComponent :type "PrimitiveComponent Object Reference") (OtherActor :type "Actor Object Reference") (OtherComp :type "PrimitiveComponent Object Reference") (OtherBodyIndex :type Integer) (bFromSweep :type Boolean) (SweepResult :type "HitResult Structure (by ref)"))
  (cast `/Game/TopDown/Blueprints/BP_TopDownCharacter` OtherActor)
  (bind _asbp_top_down_game_mode (cast `/Game/TopDown/Blueprints/BP_TopDownGameMode` (`GameplayStatics.GetGameMode`)))
  (`/Game/TopDown/Blueprints/BP_TopDownGameMode.Respawn` _asbp_top_down_game_mode))

(event `Wall advance`
  (if (`self.Can Move ?`)
    (set `CharacterMovementComponent.MaxWalkSpeed` (`self.Advance speed`) (`self.CharacterMovement`))
    (`|AIMoveTo` self (`SceneComponent.K2_GetComponentLocation` (`/Game/benoit/BP_Zone_Changer.DefaultSceneRoot` (`self.Goal`))) null)))

(fn `UserConstructionScript`)