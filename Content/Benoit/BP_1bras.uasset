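; BP_1bras is an arm ("bras") pickup for the top-down character.
; On box overlap, a character whose Bras value is 0 or 1 gets RecupereBras(0), then the pickup hides its sphere and disables box collision instead of being destroyed.
; At BeginPlay it binds to the game mode's ResetDeath event, which makes the sphere visible and re-enables query collision so the pickup returns.
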(event `self.Box.OnComponentBeginOverlap`
  (params (OverlappedComponent :type "PrimitiveComponent Object Reference") (OtherActor :type "Actor Object Reference") (OtherComp :type "PrimitiveComponent Object Reference") (OtherBodyIndex :type Integer) (bFromSweep :type Boolean) (SweepResult :type "HitResult Structure (by ref)"))
  (bind _asbp_top_down_character (cast `/Game/TopDown/Blueprints/BP_TopDownCharacter` OtherActor))
  (bind _output_get (set `self.As BP Top Down Character` _asbp_top_down_character))
  (switch `int` (`/Game/TopDown/Blueprints/BP_TopDownCharacter.Bras?` _output_get)
    (:`0`
      _)
    (:`1`
      _))
  (`/Game/TopDown/Blueprints/BP_TopDownCharacter.RecupereBras` (`self.As BP Top Down Character`) 0)
  (`self.Arms visibility`))

(event `Arms visibility`
  (`SceneComponent.SetHiddenInGame` (`self.Sphere`) true false)
  (`PrimitiveComponent.SetCollisionEnabled` (`self.Box`) "NoCollision"))

(event `self.ReceiveBeginPlay`
  (bind _asbp_top_down_game_mode (cast `/Game/TopDown/Blueprints/BP_TopDownGameMode` (`GameplayStatics.GetGameMode`)))
  (bind _output_get (set `self.As BP Top Down Game Mode` _asbp_top_down_game_mode))
  (add `/Game/TopDown/Blueprints/BP_TopDownGameMode.Reset_death` _output_get (delegate `Reset visibility`)))

(event `Reset visibility`
  (`SceneComponent.SetHiddenInGame` (`self.Sphere`) false false)
  (`PrimitiveComponent.SetCollisionEnabled` (`self.Box`) "QueryOnly"))

(fn `UserConstructionScript`)