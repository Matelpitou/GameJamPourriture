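; BP_Kamikaze is an enemy character that patrols, detects the player and can explode, triggering a respawn through the game mode.
; It caches patrol point locations on BeginPlay and hands them out cyclically through GetNextPoint.
; Pawn sensing flags the player as seen and has AIC_kamikaze update its blackboard.
; The game mode's death-reset event clears that flag, disables attacking and stops movement.
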(event `self.ReceiveBeginPlay`
  (bind _asbp_top_down_game_mode (cast `/Game/TopDown/Blueprints/BP_TopDownGameMode` (`GameplayStatics.GetGameMode`)))
  (set `self.As BP Top Down Game Mode` _asbp_top_down_game_mode)
  (add `/Game/TopDown/Blueprints/BP_TopDownGameMode.Reset_death` (`self.As BP Top Down Game Mode`) (delegate `bind dispatcher`))
  (bind _asaic_kamikaze (cast `/Game/Benoit/Ennemies/AIC_kamikaze` (`AIBlueprintHelperLibrary.GetAIController` self)))
  (set `self.As AIC Kamikaze` _asaic_kamikaze)
  (set `/Game/Benoit/Ennemies/AIC_kamikaze.Bp_Kamikaze` self _asaic_kamikaze)
  (`/Engine/EditorBlueprintResources/StandardMacros.DoOnce` false
    (:`Completed`
      (for _array_element (`self.Patrol_points`)
        (`KismetArrayLibrary.Array_Add` (`self.Positions`) (`SceneComponent.K2_GetComponentLocation` (`/Game/Benoit/Ennemies/Patrol_Point.DefaultSceneRoot` _array_element)))))))

(event `bind dispatcher`
  (bind _as_aic_kamikaze (`self.As AIC Kamikaze`))
  (set `self.Has seen player` false)
  (`/Game/Benoit/Ennemies/AIC_kamikaze.Tell BB` (`self.As AIC Kamikaze`))
  (set `/Game/Benoit/Ennemies/AIC_kamikaze.Can attack ?` false _as_aic_kamikaze)
  (`/Game/Benoit/Ennemies/AIC_kamikaze.Can Attack` _as_aic_kamikaze)
  (`MovementComponent.StopMovementImmediately` (`self.CharacterMovement`)))

(event `self.PawnSensing.OnSeePawn`
  (params (Pawn :type "Pawn Object Reference"))
  (cast `/Game/TopDown/Blueprints/BP_TopDownCharacter` Pawn)
  (set `self.Has seen player` true)
  (`/Game/Benoit/Ennemies/AIC_kamikaze.Tell BB` (`self.As AIC Kamikaze`)))

(event `Explode`
  (`GameplayStatics.SpawnEmitterAtLocation` "/Game/RPGEffects/Particles/P_Mage_Whirlwind.P_Mage_Whirlwind" (`SceneComponent.K2_GetComponentLocation` (`self.CapsuleComponent`)) (struct) (0.5 0.5 0.5))
  (`KismetSystemLibrary.Delay` 0.2)
  (bind _asbp_top_down_game_mode (cast `/Game/TopDown/Blueprints/BP_TopDownGameMode` (`GameplayStatics.GetGameMode`)))
  (`/Game/TopDown/Blueprints/BP_TopDownGameMode.Respawn` _asbp_top_down_game_mode))

(fn `Get next point`
  (returns (NewParam :type "Vector Structure"))
  (locals (Position :type "Vector Structure"))
  (set `local.Position` (`|GetArrayItem` (`self.Positions`) (`self.Length`)))
  (bind _result (`/Engine/EditorBlueprintResources/StandardMacros.IncrementInt` (`self.Length`))
    (:`  `
      (set `self.Length` _result)
      (if (>= (`self.Length`) (`KismetArrayLibrary.Array_Length` (`self.Positions`)))
        (set `self.Length` 0))
      (return (`local.Position`)))))

(fn `UserConstructionScript`)